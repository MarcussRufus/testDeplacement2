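; BP_Slalom is a slalom obstacle Actor for Map1, built from six cone components.
; On BeginPlay, it applies its Physic variable to each cone's Simulate Physics setting, so one flag decides whether the whole set simulates physics.
; The construction script is empty, and it has no active overlap or Tick logic.
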(event EventBeginPlay
  (bind _physic (Variables|Default|Getphysic))
  (Physics|SetSimulatePhysics (Variables|Default|Getcone1) _physic)
  (Physics|SetSimulatePhysics (Variables|Default|Getcone2) _physic)
  (Physics|SetSimulatePhysics (Variables|Default|Getcone3) _physic)
  (Physics|SetSimulatePhysics (Variables|Default|Getcone4) _physic)
  (Physics|SetSimulatePhysics (Variables|Default|Getcone5) _physic)
  (Physics|SetSimulatePhysics (Variables|Default|Getcone) _physic))

(event Collision|EventActorBeginOverlap
  (params (OtherActor :type Actor%20Object%20Reference)))

(event EventTick
  (params (DeltaSeconds :type Float%20%28single-precision%29)))

(fn ConstructionScript)